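; Test Blueprint that exercises the Houdini Engine session API through node creation, wiring and cleanup.
; ActivateSession starts a server session, initializes it with cook options, loads an asset library from file and instantiates its asset.
; It adds a "ProgrammaticBox" geo child, connects it to the first existing child, cooks and queries the input.
; It then disconnects and deletes that node, saves a HIP file and cleans up the session.
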(event Custom|Activate%20Session
  (bind _returnvalue (Class|CustomHEnginePluginBPLibrary|StartServerandCreateSession (Variables|Default|GetHoudini%20Session)))
  (bind _output_get (Variables|Default|SetHoudini%20Session _returnvalue))
  (bind _returnvalue_2 (Class|CustomHEnginePluginBPLibrary|CreateHoudiniCookOptions))
  (bind _output_get_2 (Variables|Default|SetHoudiniCookOptions _returnvalue_2))
  (Class|CustomHEnginePluginBPLibrary|HoudiniInitialize _output_get _output_get_2)
  (if (Class|CustomHEnginePluginBPLibrary|HoudiniIsInitialized _output_get)
    (bind _assetlibraryid (Class|CustomHEnginePluginBPLibrary|HoudiniLoadAssetLibraryfromFile _output_get (Variables|Default|GetOtl%20File%20Path) true))
    (bind _output_get_3 (Variables|Default|SetAsset%20Library%20Id _assetlibraryid))
    (bind (_fullopname _label) (Class|CustomHEnginePluginBPLibrary|HoudiniGetAssetOperatorName _output_get _output_get_3))
    (bind _nodeid (Class|CustomHEnginePluginBPLibrary|HoudiniCreateNode _output_get _fullopname _label -1 false))
    (bind _childcount (Class|CustomHEnginePluginBPLibrary|HoudiniComposeChildNodeList _output_get _nodeid "HOUDINI_NODETYPE_ANY" "HOUDINI_NODEFLAGS_ANY" false))
    (bind _childnodeidlist (Class|CustomHEnginePluginBPLibrary|HoudiniGetComposedChildNodeList _output_get _nodeid _childcount))
    (bind _nodeid_2 (Class|CustomHEnginePluginBPLibrary|HoudiniCreateNode _output_get "geo" "ProgrammaticBox" _nodeid false))
    (Class|CustomHEnginePluginBPLibrary|HoudiniConnectNodeInput _output_get _nodeid_2 0 (Utilities|Array|Get(acopy) _childnodeidlist))
    (Class|CustomHEnginePluginBPLibrary|HoudiniCookNode _output_get _nodeid _output_get_2)
    (Class|CustomHEnginePluginBPLibrary|HoudiniQueryNodeInput _output_get _nodeid_2)
    (bind _childcount_2 (Class|CustomHEnginePluginBPLibrary|HoudiniComposeChildNodeList _output_get _nodeid "HOUDINI_NODETYPE_ANY" "HOUDINI_NODEFLAGS_ANY" false))
    (Class|CustomHEnginePluginBPLibrary|HoudiniGetComposedChildNodeList _output_get _nodeid _childcount_2)
    (Class|CustomHEnginePluginBPLibrary|HoudiniDisconnectNodeInput _output_get _nodeid_2)
    (Class|CustomHEnginePluginBPLibrary|HoudiniDeleteNode _output_get _nodeid_2)
    (Class|CustomHEnginePluginBPLibrary|HoudiniSaveHIPFile _output_get (Variables|Default|GetFile%20Path) false)
    (Class|CustomHEnginePluginBPLibrary|HoudiniCleanupSession _output_get)))

(event EventBeginPlay)

(event Collision|EventActorBeginOverlap
  (params (OtherActor :type Actor%20Object%20Reference)))

(event EventTick
  (params (DeltaSeconds :type Float%20%28single-precision%29)))

(fn ConstructionScript)