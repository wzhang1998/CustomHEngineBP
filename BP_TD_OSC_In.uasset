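; Actor that receives OSC messages and uses them to drive noise materials and lights in the level.
; On BeginPlay it starts a listening OSC server and binds a message handler that branches on the address.
; The `/dist_3D` float sets noise scale on NoiseMat actors, while the `/h2:victory` integer sets BPLight visibility.
; Both branches print the received value and find their targets by class; a ChangeSize call is left unconnected.
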(event Custom|OnMsgReceived
  (params (Message :type OSC%20Message%20Structure%20%28by%20ref%29) (IPAddress :type String) (Port :type Integer))
  ;[1 1 1] Binding to Any Message
  (bind _returnvalue (Class|OSCManager|GetOSCMessageAddress Message))
  (bind _returnvalue_2 (Class|OSCManager|GetOSCAddressFullPath _returnvalue))
  (if (Class|KismetStringLibrary|MatchesWildcard _returnvalue_2 "/dist_3D" "IgnoreCase")
    (bind _value (Class|OSCManager|GetFloat Message))
    (Development|PrintString (Utilities|String|Append "Address: " _returnvalue_2 "Value: " (Utilities|String|ToString(Float) _value)))
    (bind _outactors (Actor|GetAllActorsOfClass (Variables|Default|Getnoise_mat)))
    (Default|SetNoiseScale _outactors _value)
    (elif (Class|KismetStringLibrary|MatchesWildcard _returnvalue_2 "/h2:victory" "IgnoreCase")
      (bind _value_2 (Class|OSCManager|GetInt32 Message))
      (Development|PrintString (Utilities|String|Append "Address: " _returnvalue_2 "Value: " (Utilities|String|ToString(Integer) _value_2)))
      (bind _outactors_2 (Actor|GetAllActorsOfClass (Variables|Default|GetBP_light)))
      (Default|SetVisibility _outactors_2 _value_2))))

(event EventBeginPlay
  ;[1 1 1] Binding to Any Message
  (bind _returnvalue (Class|OSCManager|CreateOSCServer (Variables|Default|GetReceive%20IPAddress) (Variables|Default|GetPort) false true "UE_OSC" 0))
  (bind _output_get (Variables|Default|SetTD_OSC_Server _returnvalue))
  (EventDispatchers|AssignOnOscMessageReceived _output_get (delegate Custom|OnMsgReceived)))

(event Collision|EventActorBeginOverlap
  (params (OtherActor :type Actor%20Object%20Reference))
  ;[1 1 1] Binding to Any Message
)

(event EventTick
  (params (DeltaSeconds :type Float%20%28single-precision%29)))

(fn ConstructionScript)