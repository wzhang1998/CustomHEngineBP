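; Actor that round-trips a static mesh actor's geometry through a Houdini Engine digital asset and rebuilds the result as a procedural mesh.
; Activate sends mesh attributes and transform to a Houdini input node, then loads and cooks the asset.
; It reads attributes back with axis and winding conversion, creating one section per material.
; The HIP save and session cleanup sit inside the section loop; the construction script's Activate call is disconnected.
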(event Custom|Activate
  (bind _proceduralmesh (Variables|Default|GetProceduralMesh))
  (CallFunction|GetMeshData (Variables|Default|GetStaticMeshActor))
  (if (Class|CustomHEnginePluginBPLibrary|HoudiniIsSessionValid (Variables|Default|GetHoudini%20Session))
    _
    (else
      (bind _returnvalue (Class|CustomHEnginePluginBPLibrary|StartServerandCreateSession (Variables|Default|GetHoudini%20Session)))
      (Variables|Default|SetHoudini%20Session _returnvalue)))
  (if (Class|CustomHEnginePluginBPLibrary|HoudiniIsInitialized (Variables|Default|GetHoudini%20Session))
    _
    (else
      (Class|CustomHEnginePluginBPLibrary|HoudiniInitialize (Variables|Default|GetHoudini%20Session) (Variables|Default|GetHoudini%20Cook%20Options))))
  (bind _nodeid (Class|CustomHEnginePluginBPLibrary|HoudiniCreateInputNode (Variables|Default|GetHoudini%20Session) "TestUnrealMesh"))
  (bind _output_get (Variables|Default|SetNode%20Id _nodeid))
  (Class|CustomHEnginePluginBPLibrary|HoudiniSetOBJNodeTransform (Variables|Default|GetHoudini%20Session) (.ParentNodeId (Class|CustomHEnginePluginBPLibrary|HoudiniGetNodeInfoSubData (.NodeInfo (Class|CustomHEnginePluginBPLibrary|HoudiniGetNodeInfo (Variables|Default|GetHoudini%20Session) _output_get)))) (Transformation|GetActorTransform (Variables|Default|GetStaticMeshActor)))
  (CallFunction|HoudiniCreateandSetPartInfo (Variables|Default|GetHoudini%20Session) _output_get (Utilities|Array|Length (Variables|Default|GetFace%20List)) (Utilities|Array|Length (Variables|Default|GetVertex%20List)) (Utilities|Array|Length (Variables|Default|GetPosition%20List)) "HOUDINI_PARTTYPE_MESH")
  (CallFunction|HoudiniSetupBaseAttribute (Variables|Default|GetHoudini%20Session) _output_get (Variables|Default|GetPosition%20List) (Variables|Default|GetNormal%20List) (Variables|Default|GetUV%20List) (Variables|Default|GetTangent%20List) (Variables|Default|GetSection%20Index%20List) (Variables|Default|GetVertex%20List))
  (Class|CustomHEnginePluginBPLibrary|HoudiniCommitGeo (Variables|Default|GetHoudini%20Session) _output_get)
  (bind _assetlibraryid (Class|CustomHEnginePluginBPLibrary|HoudiniLoadAssetLibraryfromFile (Variables|Default|GetHoudini%20Session) (Variables|Default|GetOtl%20File%20Path) false))
  (bind (_fullopname _label) (Class|CustomHEnginePluginBPLibrary|HoudiniGetAssetOperatorName (Variables|Default|GetHoudini%20Session) _assetlibraryid))
  (bind _nodeid_2 (Class|CustomHEnginePluginBPLibrary|HoudiniCreateNode (Variables|Default|GetHoudini%20Session) _fullopname _label -1 false))
  (Class|CustomHEnginePluginBPLibrary|HoudiniConnectNodeInput (Variables|Default|GetHoudini%20Session) _nodeid_2 _output_get)
  (Class|CustomHEnginePluginBPLibrary|HoudiniCookNode (Variables|Default|GetHoudini%20Session) _nodeid_2 (Variables|Default|GetHoudini%20Cook%20Options))
  (bind _dataarray (CallFunction|HoudiniGetFloatAttributeData (Variables|Default|GetHoudini%20Session) _nodeid_2 0 "P" "HOUDINI_ATTROWNER_POINT"))
  (Variables|Default|SetFinalPositionList (.VectorList (Class|CustomHEngineUtilsLibrary|FloatListtoVectorList _dataarray true 1e+02)))
  (bind _dataarray_2 (CallFunction|HoudiniGetFloatAttributeData (Variables|Default|GetHoudini%20Session) _nodeid_2 0 "N" "HOUDINI_ATTROWNER_POINT"))
  (Variables|Default|SetFinalNormalList (.VectorList (Class|CustomHEngineUtilsLibrary|FloatListtoVectorList _dataarray_2 true 1.0)))
  (bind _dataarray_3 (CallFunction|HoudiniGetFloatAttributeData (Variables|Default|GetHoudini%20Session) _nodeid_2 0 "uv" "HOUDINI_ATTROWNER_POINT"))
  (Variables|Default|SetFinalUVList (.Vector2DList (Class|CustomHEngineUtilsLibrary|FloatListtoVector2DList _dataarray_3 true)))
  (bind _dataarray_4 (CallFunction|HoudiniGetFloatAttributeData (Variables|Default|GetHoudini%20Session) _nodeid_2 0 "Tangent" "HOUDINI_ATTROWNER_POINT"))
  (Variables|Default|SetFinalProcMeshTangentList (.ProcMeshTangentList (Class|CustomHEngineUtilsLibrary|FloatListtoProcMeshTangentList _dataarray_4 true false)))
  (bind _dataarray_5 (CallFunction|HoudiniGetIntAttributeData (Variables|Default|GetHoudini%20Session) _nodeid_2 0 "SectionIndex" "HOUDINI_ATTROWNER_PRIM"))
  (bind _output_get_2 (Variables|Default|SetFinalSectionIndexList _dataarray_5))
  (bind _output_get_3 (Variables|Default|SetFinalVertexList (.VertexList (Class|CustomHEnginePluginBPLibrary|HoudiniGetVertexList (Variables|Default|GetHoudini%20Session) _nodeid_2 0 (* (.FaceCount (Class|CustomHEnginePluginBPLibrary|HoudiniGetPartInfoSubdata (.PartInfo (Class|CustomHEnginePluginBPLibrary|HoudiniGetPartInfo (Variables|Default|GetHoudini%20Session) _nodeid_2)))) 3)))))
  (Class|CustomHEngineUtilsLibrary|ReverseVertexListOrder _output_get_3)
  (for (_array_element _array_index) (.SplittedVertexLists (Class|CustomHEngineUtilsLibrary|SplitVertexList _output_get_3 _output_get_2))
    (Class|ProceduralMeshComponent|CreateMeshSectionLinearColor _proceduralmesh _array_index (Variables|Default|GetFinalPositionList) (Utilities|Struct|BreakVertexListStruct _array_element) (Variables|Default|GetFinalNormalList) (Variables|Default|GetFinalUVList) 0 0 0 0 (Variables|Default|GetFinalProcMeshTangentList) false false)
    (Rendering|Material|SetMaterial _proceduralmesh _array_index (Utilities|Array|Get(acopy) (Variables|Default|GetMaterial%20List) _array_index))
    (Class|CustomHEnginePluginBPLibrary|HoudiniSaveHIPFile (Variables|Default|GetHoudini%20Session) (Variables|Default|GetFile%20Path) false)
    (Class|CustomHEnginePluginBPLibrary|HoudiniCleanupSession (Variables|Default|GetHoudini%20Session))))

(fn ConstructionScript)

(fn GetMeshData
  (params (StaticMeshActor :type Static%20Mesh%20Actor%20Object%20Reference))
  (bind _staticmeshcomponent (Variables|/Script/Engine.StaticMeshActor|GetStaticMeshComponent StaticMeshActor))
  (bind _staticmesh (Variables|/Script/Engine.StaticMeshComponent|GetStaticMesh _staticmeshcomponent))
  (bind (_positionlist _vertexlist _facelist _normallist _tangentlist _uvlist _sectionindexlist _materiallist _returnvalue) (Class|CustomHEngineUtilsLibrary|GetUnrealMeshData _staticmesh))
  (if _returnvalue
    (Variables|Default|SetPosition%20List _positionlist)
    (Variables|Default|SetVertex%20List _vertexlist)
    (Variables|Default|SetFace%20List _facelist)
    (Variables|Default|SetNormal%20List _normallist)
    (Variables|Default|SetTangent%20List _tangentlist)
    (Variables|Default|SetUV%20List _uvlist)
    (Variables|Default|SetSection%20Index%20List _sectionindexlist)
    (Variables|Default|SetMaterial%20List _materiallist)))