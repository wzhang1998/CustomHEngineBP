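; Actor Blueprint that exposes runtime control over the material noise and size of its Sphere component.
; The construction script applies the NoiseScale variable to the "Noise Scale" scalar parameter on the sphere's materials.
; SetNoiseScale pushes a new value straight to that parameter without updating the variable, and ChangeSize sets the sphere's relative scale from ObjectScale.
; No caller appears in the graph, and BeginPlay, overlap and Tick are unused.
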(event Custom|SetNoiseScale
  (params (Scale :type Float%20%28double-precision%29))
  (Rendering|Material|SetScalarParameterValueonMaterials (Variables|Default|GetSphere) "Noise Scale" Scale))

(event Custom|ChangeSize
  (params (ObjectScale :type Float%20%28double-precision%29))
  (Transformation|SetRelativeScale3D (Variables|Default|GetSphere) (Math|Conversions|ToVector(Float) ObjectScale)))

(event EventBeginPlay)

(event Collision|EventActorBeginOverlap
  (params (OtherActor :type Actor%20Object%20Reference)))

(event EventTick
  (params (DeltaSeconds :type Float%20%28single-precision%29)))

(fn ConstructionScript
  (Rendering|Material|SetScalarParameterValueonMaterials (Variables|Default|GetSphere) "Noise Scale" (Variables|Default|GetNoise%20Scale)))