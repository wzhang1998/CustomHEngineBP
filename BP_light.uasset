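; BP_light is a rect light actor set up for Remote Control, using a preset named Remote_MIDI_test.
; SetVisibility shows the light when its integer input equals 1 and hides it below 1.
; The construction script derives a fully saturated color from ColorH and switches the editor viewport between Path Tracing and Lit based on Pathtracing.
; An expose function registers a property from every BP_light in the preset's "lights" group, labeled by actor name.
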(event Custom|SetVisibility
  (params (Light_Event :type Integer))
  (bind _rectlight (Variables|Default|GetRectLight))
  (Math|Integer|CompareInt Light_Event 1
    (:==
      (Rendering|SetVisibility _rectlight true false))
    (:<
      (Rendering|SetVisibility _rectlight false false))))

(event EventBeginPlay)

(event Collision|EventActorBeginOverlap
  (params (OtherActor :type Actor%20Object%20Reference)))

(event EventTick
  (params (DeltaSeconds :type Float%20%28single-precision%29)))

(fn ConstructionScript
  (Rendering|Components|Light|SetLightColor (Variables|Default|GetRectLight) (Class|KismetMathLibrary|HSVtoRGB (Variables|Default|GetColor_H) 1.0 1.0 1.0) true)
  (if (Variables|Default|GetPathtracing)
    (Class|AutomationBlueprintFunctionLibrary|SetEditorViewportViewMode "VMI_PathTracing")
    (else
      (Class|AutomationBlueprintFunctionLibrary|SetEditorViewportViewMode "VMI_Lit"))))

(fn ExposeAllParameters
  (bind _outactors (Actor|GetAllActorsOfClass "BP_light_C"))
  (for _array_element _outactors
    (Class|RemoteControlFunctionLibrary|ExposeProperty "/Game/BP/Remote_MIDI_test.Remote_MIDI_test" _array_element "" (Utilities|Struct|MakeRemoteControlOptionalExposeArgs (Utilities|String|Append "" (Utilities|GetDisplayName _array_element)) "lights"))))